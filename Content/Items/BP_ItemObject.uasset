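; BP_ItemObject describes an item through its icon, dimensions, class and data, exposed by getter functions.
; GetIcon returns IconRotated or Icon depending on the Rotated flag, while GetDimensions returns the stored Dimensions without checking rotation.
; GetItemClass and GetItemData return their stored variables directly, and SetItemData is an empty stub.
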(fn `Get Icon`
  (returns (Icon :type "MaterialInterface Object Reference"))
  (return (select `bool` (`self.Rotated`) :`false` (`self.Icon`) :`true` (`self.IconRotated`))))

(fn `GetDimensions`
  (returns (Dimensions :type "IntPoint Structure"))
  (return (`self.Dimensions`)))

(fn `GetItemClass`
  (returns (ItemClass :type "/Game/Items/BP_Item Class Reference"))
  (return (`self.ItemClass`)))

(fn `GetItemData`
  (returns (ItemData :type "/Game/Structures/ST_Item Structure"))
  (return (`self.ItemData`)))

(fn `SetItemData`)